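; MyCharacter_BP is a player character Blueprint handling movement, camera look and limited multi-jump.
; Movement axes apply fixed-step local offsets along pitch-only control-rotation vectors, with sweep set by IsSweep, bypassing movement input and delta-time scaling.
; Camera axes feed controller yaw and pitch.
; A DoN gate caps jumps at JumpMaxCount and resets on landing, while releasing the key stops jumping.
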(event `InputAxis|前後`
  (params (AxisValue :type "Float (single-precision)"))
  (`self.K2_AddActorLocalOffset` (* (* (`KismetMathLibrary.GetForwardVector` (`KismetMathLibrary.MakeRotator` 0.0 (.pitch (`self.GetControlRotation`)))) AxisValue) 3.0) (`self.IsSweep`)))

(event `InputAxis|左右`
  (params (AxisValue :type "Float (single-precision)"))
  (`self.K2_AddActorLocalOffset` (* (* (`KismetMathLibrary.GetRightVector` (`KismetMathLibrary.MakeRotator` 0.0 (.pitch (`self.GetControlRotation`)))) AxisValue) 3.0) (`self.IsSweep`)))

(event `InputAxis|カメラ回転_左右`
  (params (AxisValue :type "Float (single-precision)"))
  (`self.AddControllerYawInput` AxisValue))

(event `InputAction|IsJump`
  (params (Key :type "Key Structure"))
  (:`Pressed`
    (`/Engine/EditorBlueprintResources/StandardMacros.Do N` (`self.JumpMaxCount`) :!label _label
      (:`Exit`
        (`self.Jump`))))
  (:`Released`
    (`self.StopJumping`)))

(event `InputAxis|カメラ回転_上下`
  (params (AxisValue :type "Float (single-precision)"))
  (`self.AddControllerPitchInput` AxisValue))

(event `self.OnLanded`
  (params (Hit :type "HitResult Structure (by ref)"))
  (goto _label :!via `Reset`))

(event `InputAction|IsRun`
  (params (Key :type "Key Structure")))

(fn `UserConstructionScript`)