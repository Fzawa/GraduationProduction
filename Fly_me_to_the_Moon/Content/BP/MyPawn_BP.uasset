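; MyPawn_BP is a player pawn that moves and rotates from four input axes: forward/back, left/right, and horizontal and vertical camera rotation.
; Movement adds local offsets without sweep, along forward and right vectors built from control-rotation pitch alone.
; Rotation adds local yaw or pitch, both derived from control-rotation pitch rather than a fixed rate.
; All four handlers scale by axis value, delta time and a shared constant.
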(event `InputAxis|前後`
  (params (AxisValue :type "Float (single-precision)"))
  (`self.K2_AddActorLocalOffset` (* (`KismetMathLibrary.GetForwardVector` (`KismetMathLibrary.MakeRotator` 0.0 (.pitch (`self.GetControlRotation`)))) (* AxisValue (`GameplayStatics.GetWorldDeltaSeconds`) 500.0))))

(event `InputAxis|左右`
  (params (AxisValue :type "Float (single-precision)"))
  (`self.K2_AddActorLocalOffset` (* (`KismetMathLibrary.GetRightVector` (`KismetMathLibrary.MakeRotator` 0.0 (.pitch (`self.GetControlRotation`)))) (* AxisValue (`GameplayStatics.GetWorldDeltaSeconds`) 500.0))))

(event `InputAxis|カメラ回転_左右`
  (params (AxisValue :type "Float (single-precision)"))
  (`self.K2_AddActorLocalRotation` (* (`KismetMathLibrary.MakeRotator` 0.0 0.0 (.pitch (`self.GetControlRotation`))) (* AxisValue (`GameplayStatics.GetWorldDeltaSeconds`) 500.0))))

(event `InputAxis|カメラ回転_上下`
  (params (AxisValue :type "Float (single-precision)"))
  (`self.K2_AddActorLocalRotation` (* (`KismetMathLibrary.MakeRotator` 0.0 (.pitch (`self.GetControlRotation`))) (* AxisValue (`GameplayStatics.GetWorldDeltaSeconds`) 500.0))))

(fn `UserConstructionScript`)